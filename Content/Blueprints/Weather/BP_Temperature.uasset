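; BP_Temperature computes a world temperature that varies over the day and shows it on the player's cold UI widget.
; A looping timer, paced by the update rate, samples a fluctuation curve at the wrapped fraction of the day, then scales it and offsets it by a base temperature.
; The widget reference comes from the ThirdPersonCharacter's HUD.
; Day length derives from minutes in the construction script, while elapsed time is only read here.
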(event `self.ReceiveBeginPlay`
  (`|ExecutionSequence`
    (:`then_0`
      (`self.SetHUDRef`))
    (:`then_1`
      (`self.UpdateTemperature`))))

(fn `GetFractionOfDay`
  (returns (ReturnValue :type "Float (double-precision)"))
  (return (/ (`self.ElapsedTime`) (`self.Sec/day`))))

(fn `SetHUDRef`
  (`/Engine/EditorBlueprintResources/StandardMacros.IsValid` (`self.UI ColdREf`)
    (:`Is Not Valid`
      (bind _asthird_person_character (cast `/Game/ThirdPersonBP/Blueprints/ThirdPersonCharacter` (`GameplayStatics.GetPlayerCharacter` 0)))
      (set `self.UI ColdREf` (`/Game/UMGs/UMG_PlayerHUD.UI_Cold` (`/Game/ThirdPersonBP/Blueprints/ThirdPersonCharacter.HUD Ref` _asthird_person_character))))))

(fn `UpdateTemperature`
  (`KismetSystemLibrary.K2_SetTimer` self "WorldTemperature" (/ 1.0 (`self.TemperatureUpdateRate`)) true))

(fn `UserConstructionScript`
  (set `self.Sec/day` (* (`self.Minutes/Day`) 60.0)))

(fn `WorldTemperature`
  (bind _output_get (set `self.FinalWorldTemperature` (+ (* (`CurveFloat.GetFloatValue` (`self.TemperatureFluctuation`) (mod (`self.GetFractionOfDay`) 1.0)) (`self.WorldTemperatureVariation`)) (`self.BaseTemperature`))))
  (`/Game/UMGs/UI_Cold.SetWorldTemp` (`self.UI ColdREf`) _output_get (`self.DegreeType`)))